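; BP_UCharacter is a character Blueprint that wires debug display and test inputs to its buff, state and property managers.
; BeginPlay creates a hidden PropertyDebugPanel widget, shown while Tab is held.
; Key 1 applies the YinYangBP buff to itself; key 2 alternates two common-attack indices in StateManager, then calls GaveAttackDamage on PropertyManager.
; Buff run and finish events print placeholder messages, while crit and value-change handlers are empty.
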(event `self.ReceiveBeginPlay`
  (bind _returnvalue (`|CreateWidget` "/Game/Private/UExplorer/Blueprints/Widget/PropertyDebugPanel.PropertyDebugPanel_C"))
  (`UserWidget.AddToViewport` _returnvalue 0)
  (bind _output_get (set `self.DebugWidget` _returnvalue))
  (`Widget.SetVisibility` _output_get "Hidden"))

(event `Key|Tab`
  (params (Key :type "Key Structure"))
  (bind _debugwidget (`self.DebugWidget`))
  (:`Pressed`
    (`Widget.SetVisibility` _debugwidget "Visible"))
  (:`Released`
    (`Widget.SetVisibility` _debugwidget "Hidden")))

(event `self.BuffManager.BuffRunEvent`
  (params (BuffClass :type "BuffBase Class Reference"))
  (`KismetSystemLibrary.PrintString` (`KismetTextLibrary.Conv_TextToString` (`|FormatText` "{Name} RunRunRun" (`KismetTextLibrary.Conv_NameToText` "None")))))

(event `self.BuffManager.BuffFinishedEvent`
  (params (BuffClass :type "BuffBase Class Reference"))
  (`KismetSystemLibrary.PrintString` (`KismetTextLibrary.Conv_TextToString` (`|FormatText` "{Name} FinishedFishend" (`KismetTextLibrary.Conv_NameToText` "None")))))

(event `Key|One`
  (params (Key :type "Key Structure"))
  (:`Pressed`
    (`BuffManager.AcquiredBuff` (`self.BuffManager`) "/Game/Private/UExplorer/Blueprints/Buff/YinYangBP.YinYangBP_C" self self)))

(event `Key|Two`
  (params (Key :type "Key Structure"))
  (bind _statemanager (`self.StateManager`))
  (:`Pressed`
    (`/Engine/EditorBlueprintResources/StandardMacros.FlipFlop`
      (:`A`
        (`StateManager.SetCombatState` _statemanager "CommonAtk" 1))
      (:`B`
        (`StateManager.SetCombatState` _statemanager "CommonAtk" 2)))
    (`PropertyManager.GaveAttackDamage` (`self.PropertyManager`))))

(event `self.PropertyManager.CritEvent`
  (params (bIsCrit :type Boolean) (DamageType :type "EDamageType Enum" :default "PhysicalDamage")))

(event `self.PropertyManager.ValueChangedEvent`
  (params (ChangedValueType :type "EPropertyValueType Enum" :default "InitValue")))

(fn `UserConstructionScript`
  (`parent.UserConstructionScript`))