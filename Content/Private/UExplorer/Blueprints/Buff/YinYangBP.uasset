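; YinYang buff actor that so far only prints debug messages, with no gameplay effect.
; It overrides the buff lifecycle functions, each advancing the state from waiting through running and finished to dead, then destroying the actor.
; The running step prints repeatedly in a single loop and finishes immediately, and the event graph holds only disabled default nodes.
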(fn `BuffAwake`
  (returns (ReturnValue :type Boolean))
  (`self.SetBuffState` "Waiting")
  (return false))

(fn `BuffDestroy`
  (returns (ReturnValue :type Boolean))
  (`self.K2_DestroyActor`)
  (return false))

(fn `BuffFinished`
  (returns (ReturnValue :type Boolean))
  (`self.SetBuffState` "Dead")
  (return false))

(fn `BuffRunning`
  (returns (ReturnValue :type Boolean))
  (for _ (range 11)
    (`KismetSystemLibrary.PrintString` "YinYangRun"))
  (`self.SetBuffState` "Finished")
  (return false))

(fn `BuffStart`
  (returns (ReturnValue :type Boolean))
  (`KismetSystemLibrary.PrintString` "YinYang Start")
  (`self.SetBuffState` "Running")
  (return false))

(fn `UserConstructionScript`)