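; Pixel-style 2D player character that maps gamepad input events to movement, melee attack and weapon switching.
; Left-stick X drives scaled horizontal movement, while button presses trigger dash and jump, all through the base movement component.
; Another button calls a melee attempt on the attack component, and a FlipFlop toggles WeaponType between two values.
; Tick, overlap and construction add no custom logic.
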(event `AllInputEventsInterface.BP_LStickAxisEvent_X`
  (params (ValueX :type "Float (single-precision)"))
  (`parent.BP_LStickAxisEvent_X` ValueX)
  (`BP_MovementComponentBase.Move` (`self.BP_MovementComponentBase`) self (* ValueX 0.6)))

(event `AllInputEventsInterface.BP_LightPressStartEvent_RB`
  (`BP_MovementComponentBase.Dash` (`self.BP_MovementComponentBase`) 800.0 0.3))

(event `AllInputEventsInterface.BP_LightPressStartEvent_RBG_DOWN`
  (`BP_MovementComponentBase.Jump` (`self.BP_MovementComponentBase`) 400.0))

(event `AllInputEventsInterface.BP_LightPressStartEvent_RBG_LEFT`
  (`BP_AttackComponentBase.TryMeleeAttack` (`self.BP_AttackComponentBase`)))

(event `AllInputEventsInterface.BP_LightPressStartEvent_RBG_TOP`
  (`/Engine/EditorBlueprintResources/StandardMacros.FlipFlop`
    (:`A`
      (set `self.WeaponType` 0))
    (:`B`
      (set `self.WeaponType` 1))))

(fn `UserConstructionScript`
  (`parent.UserConstructionScript`))