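; Base AI monster pawn that shows flipbook animations matching its monster ID and movement state.
; A looping timer checks velocity to switch between two states, and an event fires whenever the state changes.
; That event looks up the monster's row in DT_AllMonsterAnimations and applies the state's flipbook to PixelComponent.
; Changing the monster ID resets the state to the low-speed one, refreshing the flipbook only if the state differs.
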(event `self.ReceiveBeginPlay`
  (`PaperFlipbookComponent.SetFlipbook` (`self.PixelComponent`) "/Game/Public/Art_Asset/Animation/EnemyAnimation/FireGun/PFB_FireGunIdle_01.PFB_FireGunIdle_01")
  (add `self.StateChangedEvent` (delegate `WhenStateChanged`))
  (add `self.IDchangedEvent` (delegate `WhenIDChanged`))
  (`KismetSystemLibrary.K2_SetTimerDelegate` (delegate `UpdateState`) 0.1 true))

(event `WhenStateChanged`
  (`self.SetCurrentAnimation`))

(event `UpdateState`
  (if (>= (`KismetMathLibrary.VSize` (`MovementComponent.Velocity` (`self.CharacterMovement`))) 10.0)
    (`self.SetMonsterState` "NewEnumerator1")
    (else
      (`self.SetMonsterState` "NewEnumerator0"))))

(event `WhenIDChanged`
  (`self.SetMonsterState` "NewEnumerator0"))

(fn `SetCurrentAnimation`
  (bind _returnvalue (`|GetDataTableRow` "/Game/Private/Sigua/DT_AllMonsterAnimations.DT_AllMonsterAnimations" (`self.CurrentMonsterRowID`))
    (:`then`
      (bind (_value _returnvalue_2) (`BlueprintMapLibrary.Map_Find` (`.MonsterStateFlipbook_16_CD6D11344F5EE5C7208885AA968FC7F2` (break `/Game/Private/Sigua/STR_MonsterAimationTableInfo` _returnvalue)) (`self.CurrentState`)))
      (if _returnvalue_2
        (`PaperFlipbookComponent.SetFlipbook` (`self.PixelComponent`) _value)))))

(fn `SetMonsterID`
  (params (MonsterID :type Name))
  (if (not (== MonsterID (`self.CurrentMonsterRowID`)))
    (set `self.CurrentMonsterRowID` MonsterID)
    (`self.IDchangedEvent`)))

(fn `SetMonsterState`
  (params (InState :type "/Game/Private/Sigua/E_NormalOnLandEnemyState Enum" :default "NewEnumerator0"))
  (if (not (`|EnumEquality` InState (`self.CurrentState`)))
    (set `self.CurrentState` InState)
    (`self.StateChangedEvent`)))

(fn `UserConstructionScript`)