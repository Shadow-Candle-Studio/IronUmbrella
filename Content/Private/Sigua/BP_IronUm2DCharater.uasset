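; BP_IronUm2DCharater is a 2D character Blueprint that turns controller input events into movement, double jump and melee attack.
; Left stick X calls the parent handler, then drives the movement component at a reduced scale.
; The bottom button reads the movement component's jump count to fire a stronger first jump or a weaker second one.
; The left button triggers a melee attempt on the attack component.
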(event `AllInputEventsInterface.BP_LightPressStartEvent_RBG_LEFT`
  ;[1 1 1] Attack Event
  (`BP_AttackComponentBase.TryMeleeAttack` (`self.BP_AttackComponentBase`)))

(event `AllInputEventsInterface.BP_LStickAxisEvent_X`
  (params (ValueX :type "Float (single-precision)"))
  ;[1 1 1] Basic MovementEvent
  (`parent.BP_LStickAxisEvent_X` ValueX)
  (`BP_MovementComponentBase.Move` (`self.BP_MovementComponentBase`) self (* ValueX 0.6)))

(event `AllInputEventsInterface.BP_LightPressStartEvent_RBG_DOWN`
  (bind _bp_movementcomponentbase (`self.BP_MovementComponentBase`))
  (bind _jumpcount (`BP_MovementComponentBase.JumpCount` _bp_movementcomponentbase))
  ;[1 1 1] JumpEvent
  (if (== 0 _jumpcount)
    ;[1 1 1] Fisrt jump
    (`BP_MovementComponentBase.Jump` _bp_movementcomponentbase 360.0)
    (elif (== _jumpcount 1)
      ;[1 1 1] Second Jump
      (`BP_MovementComponentBase.Jump` _bp_movementcomponentbase 300.0))))

(fn `UserConstructionScript`
  (`parent.UserConstructionScript`))