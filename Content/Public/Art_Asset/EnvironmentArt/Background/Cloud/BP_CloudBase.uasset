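; BP_CloudBase is a base actor for drifting background cloud sprites with a limited lifetime.
; On BeginPlay it gives the TCloudSprite component a random sprite from the Clouds array, then destroys itself after a Duration delay.
; Each Tick it moves the sprite by a Speed offset, which is not scaled by delta time, so drift speed follows frame rate.
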(event `self.ReceiveBeginPlay`
  (`PaperSpriteComponent.SetSprite` (`self.T_Cloud_Sprite`) (`KismetArrayLibrary.Array_Random` (`self.Clouds`)))
  (`KismetSystemLibrary.Delay` (`self.Duration`))
  (`self.K2_DestroyActor`))

(event `self.ReceiveTick`
  (params (DeltaSeconds :type "Float (single-precision)"))
  (`SceneComponent.K2_AddWorldOffset` (`self.T_Cloud_Sprite`) (`self.Speed`) false false))

(fn `UserConstructionScript`)