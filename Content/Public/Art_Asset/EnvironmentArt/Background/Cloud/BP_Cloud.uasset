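; BP_Cloud is a spawner actor that continuously emits BP_CloudBase actors as clouds for the background environment.
; From BeginPlay it runs an endless spawn loop, waiting SpawnDuration between clouds.
; Each cloud appears at the spawner's X with slight Y jitter and a random world Z between MinHeight and MaxHeight.
; The spawner passes each cloud a random X speed within its configured range and a shared Duration.
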(event `self.ReceiveBeginPlay`
  (bind (_returnvalue_x _returnvalue_y) (`KismetMathLibrary.BreakVector` (`self.K2_GetActorLocation`)))
  (`|SpawnActorFromClass` "/Game/Public/Art_Asset/EnvironmentArt/Background/Cloud/BP_CloudBase.BP_CloudBase_C" (`KismetMathLibrary.MakeTransform` (`KismetMathLibrary.MakeVector` _returnvalue_x (+ _returnvalue_y (`KismetMathLibrary.RandomFloatInRange` -5.0 5.0)) (`KismetMathLibrary.RandomFloatInRange` (`self.MinHeight`) (`self.MaxHeight`)))) "Undefined" "OverrideRootScale" null (`KismetMathLibrary.MakeVector` (`KismetMathLibrary.RandomFloatInRange` (`self.MinSpeed`) (`self.MaxSpeed`))) (`self.Duration`) null :!label _label)
  (`KismetSystemLibrary.Delay` (`self.SpawnDuration`))
  (goto _label))

(fn `UserConstructionScript`)