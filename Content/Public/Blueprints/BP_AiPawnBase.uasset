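; Base AI monster for a side-view flipbook game that chases BP_Hero horizontally and switches to an attack state within range.
; Each AI component loop update checks player distance, then either sets the attack state or sets X velocity, sprite facing and move/idle state.
; State and monster ID setters broadcast only on change; ID changes request idle, and state changes pick the flipbook from DT_AllMonsterAnimations by ID and state.
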(event `WhenStateChanged`
  (`self.SetCurrentAnimation`))

(event `WhenIDChanged`
  (`self.SetMonsterState` "NewEnumerator0"))

(event `self.ReceiveBeginPlay`
  (`PaperFlipbookComponent.SetFlipbook` (`self.PixelComponent`) "/Game/Public/Art_Asset/Animation/EnemyAnimation/FireGun/PFB_FireGunIdle_01.PFB_FireGunIdle_01")
  (add `self.StateChangedEvent` (delegate `WhenStateChanged`))
  (add `self.IDchangedEvent` (delegate `WhenIDChanged`)))

(event `self.BP_SimpleAiComponentBase.AiLoopUpdatedEvent`
  (bind (_getdistancesuccess _dist) (`self.GetPlayerDistance`))
  (bind _bp_simpleaicomponentbase (`self.BP_SimpleAiComponentBase`))
  (bind _asbp_hero (cast `/Game/Public/Blueprints/BP_Hero` (`SimpleAIComponentBase.GetPlayerPointer` (`self.BP_SimpleAiComponentBase`))))
  (`|ExecutionSequence`
    (:`then_0`
      (if (and _getdistancesuccess (<= _dist (`SimpleAIComponentBase.AcceptableAttackingRadius` (`self.BP_SimpleAiComponentBase`))))
        (`self.SetMonsterState` "NewEnumerator2")
        (elif (`KismetSystemLibrary.IsValid` _asbp_hero)
          (bind (_returnvalue_x _returnvalue_y _returnvalue_z) (`KismetMathLibrary.BreakVector` (- (`self.K2_GetActorLocation` _asbp_hero) (`self.K2_GetActorLocation`))))
          (bind _returnvalue_x_2 (`KismetMathLibrary.BreakVector` (`KismetMathLibrary.Normal` (`KismetMathLibrary.MakeVector` _returnvalue_x 0.0 _returnvalue_z))))
          (bind _returnvalue (* (`SimpleAIComponentBase.AiUpdateTimerSpeed` _bp_simpleaicomponentbase) (`SimpleAIComponentBase.MovingInputAdditionMultiplier` _bp_simpleaicomponentbase) _returnvalue_x_2))
          (set `MovementComponent.Velocity` (`KismetMathLibrary.MakeVector` _returnvalue) (`self.CharacterMovement`))
          (`self.AutoAdaptSpriteToVelocityDirection` _returnvalue)
          (if (>= (`KismetMathLibrary.VSize` (`MovementComponent.Velocity` (`self.CharacterMovement`))) 10.0)
            (`self.SetMonsterState` "NewEnumerator1")
            (else
              (`self.SetMonsterState` "NewEnumerator0"))))))))

(fn `GetPlayerDistance`
  (returns (GetDistanceSuccess :type Boolean) (Dist :type "Float (double-precision)"))
  (bind _returnvalue (`SimpleAIComponentBase.GetPlayerPointer` (`self.BP_SimpleAiComponentBase`)))
  (`/Engine/EditorBlueprintResources/StandardMacros.IsValid` _returnvalue
    (:`Is Valid`
      (return true (`KismetMathLibrary.Vector_Distance` (`self.K2_GetActorLocation`) (`self.K2_GetActorLocation` _returnvalue))))
    (:`Is Not Valid`
      (return false -1.0))))

(fn `SetCurrentAnimation`
  (bind _returnvalue (`|GetDataTableRow` "/Game/Private/Sigua/DT_AllMonsterAnimations.DT_AllMonsterAnimations" (`self.CurrentMonsterRowID`))
    (:`then`
      (bind (_value _returnvalue_2) (`BlueprintMapLibrary.Map_Find` (`.MonsterStateFlipbook_16_CD6D11344F5EE5C7208885AA968FC7F2` (break `/Game/Public/Blueprints/STR_MonsterAimationTableInfo` _returnvalue)) (`self.CurrentState`)))
      (if _returnvalue_2
        (`PaperFlipbookComponent.SetFlipbook` (`self.PixelComponent`) _value)))))

(fn `SetMonsterID`
  (params (MonsterID :type Name))
  (if (not (== MonsterID (`self.CurrentMonsterRowID`)))
    (set `self.CurrentMonsterRowID` MonsterID)
    (`self.IDchangedEvent`)))

(fn `SetMonsterState`
  (params (InState :type "/Game/Public/Blueprints/E_NormalOnLandEnemyState Enum" :default "NewEnumerator0"))
  (if (not (`|EnumEquality` InState (`self.CurrentState`)))
    (set `self.CurrentState` InState)
    (`self.StateChangedEvent`)))

(fn `UserConstructionScript`)