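; BP_Hero is the player's sprite-based, side-moving hero, with running, double jump, dash, parry, combo attacks and knockback stun.
; Input events drive movement and attack components, while StateManager holds action and combat states that gate input.
; The attack-end delegate advances a timer-reset three-step combo or commits weapon switches.
; A HUD widget holds the desired Umbrella, Hammer or Fist, and switching plays a transition attack for only three directed pairs.
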(event `self.ReceiveBeginPlay`
  ;[1 1 1] Initialization of BP_Hero
  (`parent.ReceiveBeginPlay`)
  (`|ExecutionSequence`
    (:`then_1`
      (add `/Game/Public/Blueprints/CharacterBlueprint/Basics/BP_ControllableCha.UpdateCurrentState` (delegate `UpdateCurrentStateEvent`)))
    (:`then_3`
      (add `self.OnTakeAnyDamage` (delegate `Take Damage`)))))

(event `self.ReceivePossessed`
  (params (NewController :type "Controller Object Reference"))
  ;[1 1 1] Initialization of BP_Hero
  (bind _returnvalue (`|CreateWidget` "/Game/Public/Blueprints/UI/UMG_WeaponStateArea.UMG_WeaponStateArea_C" (`GameplayStatics.GetPlayerController` 0)))
  (bind _output_get (set `self.WeaponWidget` _returnvalue))
  (`UserWidget.AddToViewport` _output_get 0)
  (`/Game/Public/Blueprints/UI/UMG_WeaponStateArea.InitWeaponAreaDisplay` _output_get (`self.GetCurrentWeapon Type Directly`)))

(event `Take Damage` :!signature `self.OnTakeAnyDamage`
  (params (DamagedActor :type "Actor Object Reference") (Damage :type "Float (double-precision)") (DamageType :type "DamageType Object Reference") (InstigatedBy :type "Controller Object Reference") (DamageCauser :type "Actor Object Reference"))
  (bind _returnvalue_x (`KismetMathLibrary.BreakVector` (- (`self.K2_GetActorLocation` DamageCauser) (`self.K2_GetActorLocation`))))
  ;[1 1 1] Take Damage Events
  (bind _result (`/Engine/EditorBlueprintResources/StandardMacros.NegateFloat` _returnvalue_x)
    (:`  `
      (`self.BehaveBeingHurt` (* _result 10.0) (* _returnvalue_x 8.0))
      (`self.AutoAdaptSpriteToVelocityDirection` _returnvalue_x))))

(event `UpdateCurrentStateEvent`
  (bind _charactermovement (`self.CharacterMovement`))
  (bind _statemanager (`self.StateManager`))
  (bind _staticchavelocitystandard (`self.StaticChaVelocityStandard`))
  (bind _returnvalue (`KismetMathLibrary.VSize` (`MovementComponent.Velocity` _charactermovement)))
  (bind _returnvalue_2 (and (not (`BP_MovementComponentBase.isPawnDashing` (`self.BP_UnivMovementComponent`))) (not (`NavMovementComponent.IsFalling` _charactermovement))))
  ;[1 1 1] Update Character Start
  (if (`self.CanWeMove`)
    (`|ExecutionSequence`
      (:`then_0`
        (if (and (<= _returnvalue _staticchavelocitystandard) _returnvalue_2)
          (`StateManager.SetCurrentState` _statemanager "Idle")))
      (:`then_1`
        (if (and _returnvalue_2 (> _returnvalue _staticchavelocitystandard))
          (`StateManager.SetCurrentState` _statemanager "Running"))))))

(event `AllInputEventsInterface.BP_LStickAxisEvent_X`
  (params (ValueX :type "Float (single-precision)"))
  ;[1 1 1] Basic MovementEvent
  (`parent.BP_LStickAxisEvent_X` ValueX)
  (if (`self.CanWeMove`)
    (`BP_MovementComponentBase.Move` (`self.BP_UnivMovementComponent`) self (* ValueX 0.6))))

(event `AllInputEventsInterface.BP_LightPressStartEvent_RBG_DOWN`
  (bind _bp_univmovementcomponent (`self.BP_UnivMovementComponent`))
  (bind _jumpcount (`BP_MovementComponentBase.JumpCount` (`self.BP_UnivMovementComponent`)))
  ;[1 1 1] JumpEvent
  (if (`self.CanWeMove`)
    (if (== 0 _jumpcount)
      (`BP_MovementComponentBase.Jump` _bp_univmovementcomponent 360.0)
      (elif (== _jumpcount 1)
        (`BP_MovementComponentBase.Jump` _bp_univmovementcomponent 300.0)))))

(event `BehaveBeingHurt`
  (params (ImpulseVelocityX :type "Float (double-precision)") (ImpulseVelocityZ :type "Float (double-precision)"))
  ;[1 1 1] Stun
  (`StateManager.SetCurrentState` (`self.StateManager`) "Stun")
  (set `MovementComponent.Velocity` (`KismetMathLibrary.MakeVector` ImpulseVelocityX) (`self.CharacterMovement`))
  (`BP_MovementComponentBase.Jump` (`self.BP_UnivMovementComponent`) (`KismetMathLibrary.Abs` ImpulseVelocityZ)))

(event `self.BP_UnivMovementComponent.Delegate_JumpStateChanged`
  ;[1 1 1] JumpEvent
  (if (`NavMovementComponent.IsFalling` (`self.CharacterMovement`))
    (`StateManager.SetCurrentState` (`self.StateManager`) "Jumping")
    (else
      (`StateManager.SetCurrentState` (`self.StateManager`) "Idle"))))

(event `StopBehavingHurt`
  ;[1 1 1] Stun
  (`StateManager.SetCurrentState` (`self.StateManager`) "Idle"))

(event `AllInputEventsInterface.BP_LightPressStartEvent_RBG_RIGHT`
  ;[1 1 1] DashEvent
  (if (`self.CanWeMove`)
    (`BP_MovementComponentBase.Dash` (`self.BP_UnivMovementComponent`) 600.0 0.3)))

(event `self.BP_UnivMovementComponent.Delegate_DashStateChanged`
  ;[1 1 1] DashEvent
  (if (`BP_MovementComponentBase.isPawnDashing` (`self.BP_UnivMovementComponent`))
    (`StateManager.SetCurrentState` (`self.StateManager`) "Dashing")))

(event `AllInputEventsInterface.BP_LightPressStartEvent_LBG_RIGHT`
  (bind _weaponwidget (`self.WeaponWidget`))
  ;[1 1 1] Change UI desire Weapon
  (`/Engine/EditorBlueprintResources/StandardMacros.FlipFlop`
    (:`A`
      (`/Game/Public/Blueprints/UI/UMG_WeaponStateArea.SetUIDesireWeapontype` _weaponwidget "Umbrella"))
    (:`B`
      (`/Engine/EditorBlueprintResources/StandardMacros.FlipFlop`
        (:`A`
          (`/Game/Public/Blueprints/UI/UMG_WeaponStateArea.SetUIDesireWeapontype` _weaponwidget "Hammer"))
        (:`B`
          (`/Game/Public/Blueprints/UI/UMG_WeaponStateArea.SetUIDesireWeapontype` _weaponwidget "Fist"))))))

(event `AllInputEventsInterface.BP_LightPressStartEvent_RB`
  (bind _statemanager (`self.StateManager`))
  ;[1 1 1] Parry
  (if (`self.CanWeMove`)
    (`BP_AttackComponentBase.TryMeleeAttack` (`self.BP_HeroAttackComoponent`))
    (`StateManager.SetCurrentState` _statemanager "Attacking")
    (`StateManager.SetCombatState` _statemanager "Parry" 1)))

(event `AllInputEventsInterface.BP_LightPressStartEvent_RT`
  (bind _weaponwidget (`self.WeaponWidget`))
  (bind _statemanager (`self.StateManager`))
  ;[1 1 1] Execute Switching Weapon Action Animation
  (if (not (`|EnumEquality` (`/Game/Public/Blueprints/UI/UMG_WeaponStateArea.GetUiDesireWeaponType` _weaponwidget) (`/Game/Public/Blueprints/UI/UMG_WeaponStateArea.GetUICurrentWeaponType` _weaponwidget)))
    (`|ExecutionSequence`
      (:`then_0`
        (if (or (`self.SwitchingAttackActionBoolChooser` "Umbrella" "Fist") (`self.SwitchingAttackActionBoolChooser` "Fist" "Hammer") (`self.SwitchingAttackActionBoolChooser` "Hammer" "Umbrella"))
          (`BP_AttackComponentBase.TryMeleeAttack` (`self.BP_HeroAttackComoponent`))
          (`StateManager.SetCurrentState` _statemanager "Attacking")
          (`StateManager.SetCombatState` _statemanager "SwitchWeaponTransitionAtk" 1))))))

(event `ResetAttackPhase`
  ;[1 0.06799 0.1178] Attack end event
  ;;[1 1 1] Normal Attacking
  (`KismetSystemLibrary.K2_ClearAndInvalidateTimerHandle` (`self.ResetTimer`))
  (set `self.AttackingPhase` 0))

(event `self.BP_HeroAttackComoponent.FOnAttackEndEvent`
  (bind _statemanager (`self.StateManager`))
  (bind _weaponwidget (`self.WeaponWidget`))
  (bind _attackingphase (`self.AttackingPhase`))
  ;[1 0.06799 0.1178] Attack end event
  (switch `ECombatState` (`StateManager.GetCombatState` (`self.StateManager`))
    (:`CommonAtk`
      (`StateManager.SetCurrentState` (`self.StateManager`) "Idle")
      ;;[1 1 1] Normal Attacking
      (`/Engine/EditorBlueprintResources/StandardMacros.IncrementInt` _attackingphase
        (:`  `
          (switch `int` _attackingphase
            (:`1`
              (bind _returnvalue (`KismetSystemLibrary.K2_SetTimerDelegate` (delegate `ResetAttackPhase`) (`self.Attack1_ReponseTime`)))
              (set `self.ResetTimer` _returnvalue))
            (:`2`
              (bind _returnvalue_2 (`KismetSystemLibrary.K2_SetTimerDelegate` (delegate `ResetAttackPhase`) (`self.Attack2_ReponseTime`)))
              (set `self.ResetTimer` _returnvalue_2))
            (:`3`
              (set `self.AttackingPhase` 0))))))
    (:`SwitchWeaponTransitionAtk`
      ;;[1 1 1] Switch attacking
      (`WeaponComponent.ToggleWeaponById` (`self.Weapon`) (`KismetMathLibrary.Conv_IntToByte` (`/Game/Public/Blueprints/AnimBlueprint/BP_CommonLibrary.FromWeaponTypeToID` (`/Game/Public/Blueprints/UI/UMG_WeaponStateArea.GetUiDesireWeaponType` _weaponwidget))))
      (`/Game/Public/Blueprints/UI/UMG_WeaponStateArea.OverrideUICurrentWeaponType` _weaponwidget)
      (`StateManager.SetCurrentState` _statemanager "Idle"))
    (:`Parry`
      ;;[1 1 1] Parray Attacking
      (`StateManager.SetCurrentState` _statemanager "Idle"))))

(event `AllInputEventsInterface.BP_LightPressStartEvent_RBG_LEFT`
  (bind _statemanager (`self.StateManager`))
  ;[1 0.06799 0.1178] Attack end event
  ;;[1 1 1] Normal Attack Event
  (if (`self.CanWeMove`)
    (`BP_AttackComponentBase.TryMeleeAttack` (`self.BP_HeroAttackComoponent`))
    (`PropertyManager.GaveAttackDamage` (`self.CombatValueManager`))
    (`StateManager.SetCurrentState` _statemanager "Attacking")
    (`StateManager.SetCombatState` _statemanager "CommonAtk" 1)))

(fn `CanWeMove`
  (returns (CanweMove :type Boolean))
  (bind _returnvalue (`StateManager.GetCurrentState` (`self.StateManager`)))
  (return (not (or (`|EnumEquality` _returnvalue "Attacking") (`|EnumEquality` _returnvalue "Stun") (`|EnumEquality` _returnvalue "Dead")))))

(fn `GetAttackingPhase`
  (returns (AttackingPhase :type Integer))
  (return (`self.AttackingPhase`)))

(fn `GetCurrentWeapon Type Directly`
  (returns (WeaponType :type "EWeaponType Enum"))
  (bind (_weaponinfo_weaponname _weaponinfo_weapontype) (break `WeaponInfo` (`WeaponComponent.WeaponInfo` (`self.Weapon`))))
  (return _weaponinfo_weapontype))

(fn `GetUIDisplayedCurrentWeaponType`
  (returns (CurrentUIWeaponype :type "EWeaponType Enum"))
  (bind _weaponwidget (`self.WeaponWidget`)
    (:`then`
      (return (`/Game/Public/Blueprints/UI/UMG_WeaponStateArea.GetUICurrentWeaponType` _weaponwidget)))
    (:`else`)))

(fn `GetUIDisplayedDesiredWeaponType`
  (returns (UIdesiredWeaponType :type "EWeaponType Enum"))
  (bind _weaponwidget (`self.WeaponWidget`)
    (:`then`
      (return (`/Game/Public/Blueprints/UI/UMG_WeaponStateArea.GetUiDesireWeaponType` _weaponwidget)))
    (:`else`)))

(fn `SwitchingAttackActionBoolChooser`
  (params (CurrentUIWeaponType :type "EWeaponType Enum" :default "Dagger") (UiDesiredWeaponType :type "EWeaponType Enum" :default "Dagger"))
  (returns (Result :type Boolean))
  (return (and (`|EnumEquality` (`self.GetUIDisplayedDesiredWeaponType`) UiDesiredWeaponType) (`|EnumEquality` (`self.GetUIDisplayedCurrentWeaponType`) CurrentUIWeaponType))))

(fn `UserConstructionScript`
  (`parent.UserConstructionScript`))