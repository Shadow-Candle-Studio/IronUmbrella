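; Base Blueprint for a controllable 2D character that keeps its facing in line with horizontal movement.
; On left-stick X axis input, it checks the sign of X velocity and calls ChangeFaceDirection, storing the result in LastDirection.
; When X velocity is zero, it reapplies the stored direction so the character keeps facing the way it last moved.
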(event `AllInputEventsInterface.BP_LStickAxisEvent_X`
  (params (ValueX :type "Float (single-precision)"))
  (bind _returnvalue_x (`KismetMathLibrary.BreakVector` (`self.GetVelocity`)))
  (bind _returnvalue_x_2 (`KismetMathLibrary.BreakVector` (`self.GetVelocity`)))
  (if (> _returnvalue_x_2 0.0)
    (`self.ChangeFaceDirection` true)
    (set `self.LastDirection` true)
    (elif (< _returnvalue_x 0.0)
      (`self.ChangeFaceDirection` false)
      (set `self.LastDirection` false)
      (else
        (`self.ChangeFaceDirection` (`self.LastDirection`))))))

(fn `UserConstructionScript`)